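; BP_DamageTrap is a moving trap that damages and knocks back the player on contact.
; A looping timer alternates playing and reversing a timeline, which sets the Box's world Z at the actor's X/Y.
; Box overlap applies damage to BP_Player and launches it along the inverted impact normal with an upward boost.
; Its DoOnce resets only after a player hit, so any other overlapping actor leaves it closed.
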(event `self.ReceiveBeginPlay`
  (`KismetSystemLibrary.K2_SetTimerDelegate` (delegate `ChangeLocation`) (`self.Time`) true))

(event `ChangeLocation`
  (bind (_returnvalue_x _returnvalue_y) (`KismetMathLibrary.BreakVector` (`self.K2_GetActorLocation`)))
  (`/Engine/EditorBlueprintResources/StandardMacros.FlipFlop`
    (:`A`
      (bind (_direction _changelocation) (`Timeline|Animation` :!label _label)
        (:`Update`
          (`SceneComponent.K2_SetWorldLocation` (`self.Box`) (`KismetMathLibrary.MakeVector` _returnvalue_x _returnvalue_y _changelocation) false false))))
    (:`B`
      (goto _label :!via `Reverse`))))

(event `self.Box.OnComponentBeginOverlap`
  (params (OverlappedComponent :type "PrimitiveComponent Object Reference") (OtherActor :type "Actor Object Reference") (OtherComp :type "PrimitiveComponent Object Reference") (OtherBodyIndex :type Integer) (bFromSweep :type Boolean) (SweepResult :type "HitResult Structure (by ref)"))
  (bind (_returnvalue_x _returnvalue_y) (`KismetMathLibrary.BreakVector` (* (* (`.ImpactNormal` (`GameplayStatics.BreakHitResult` SweepResult)) -1.0) 700.0)))
  (`/Engine/EditorBlueprintResources/StandardMacros.DoOnce` false :!label _label_2
    (:`Completed`
      (bind _asbp_player (cast `/Game/Player/BP_Player` OtherActor))
      (`GameplayStatics.ApplyDamage` _asbp_player 20.0)
      (`Character.LaunchCharacter` _asbp_player (`KismetMathLibrary.MakeVector` _returnvalue_x _returnvalue_y 300.0) false false)
      (goto _label_2 :!via `Reset`))))

(fn `UserConstructionScript`)