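; BP_Wheel is a trap that carries four blade actors on a wheel.
; On BeginPlay it spawns a BP_Blades actor at each of its four Blade components and attaches it there, snapping location and rotation while keeping world scale.
; The graph contains no rotation or damage logic of its own.
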(event `self.ReceiveBeginPlay`
  (bind _blade1 (`self.Blade1`))
  (bind _blade2 (`self.Blade2`))
  (bind _blade3 (`self.Blade3`))
  (bind _blade4 (`self.Blade4`))
  (bind _returnvalue (`|SpawnActorFromClass` "/Game/Traps/BP_Blades.BP_Blades_C" (`SceneComponent.K2_GetComponentToWorld` _blade1) "Undefined" "OverrideRootScale" null null))
  (`self.K2_AttachToComponent` _returnvalue _blade1 "None" "SnapToTarget" "SnapToTarget" "KeepWorld" true)
  (bind _returnvalue_2 (`|SpawnActorFromClass` "/Game/Traps/BP_Blades.BP_Blades_C" (`SceneComponent.K2_GetComponentToWorld` _blade2) "Undefined" "OverrideRootScale" null null))
  (`self.K2_AttachToComponent` _returnvalue_2 _blade2 "None" "SnapToTarget" "SnapToTarget" "KeepWorld" true)
  (bind _returnvalue_3 (`|SpawnActorFromClass` "/Game/Traps/BP_Blades.BP_Blades_C" (`SceneComponent.K2_GetComponentToWorld` _blade3) "Undefined" "OverrideRootScale" null null))
  (`self.K2_AttachToComponent` _returnvalue_3 _blade3 "None" "SnapToTarget" "SnapToTarget" "KeepWorld" true)
  (bind _returnvalue_4 (`|SpawnActorFromClass` "/Game/Traps/BP_Blades.BP_Blades_C" (`SceneComponent.K2_GetComponentToWorld` _blade4) "Undefined" "OverrideRootScale" null null))
  (`self.K2_AttachToComponent` _returnvalue_4 _blade4 "None" "SnapToTarget" "SnapToTarget" "KeepWorld" true))

(fn `UserConstructionScript`)